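; OpenDoorBP is a component that swings its owning door actor open while the player pawn overlaps an assigned PressurePlate.
; BeginPlay caches the starting yaw, treats the target yaw as an offset from it, and prints an error if the plate is missing.
; Tick calls OpenDoor during overlap and CloseDoor after a delay, each easing yaw with a delta-time-scaled Lerp.
; Comments note C++ equivalents of several nodes.
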(event EventBeginPlay
  (Variables|Default|SetDoorInitialYaw (.yaw (Transformation|GetActorRotation (Components|GetOwner))))
  (Variables|Default|SetDoorCurrentYaw (Variables|Default|GetDoorInitialYaw))
  (Variables|Default|SetDoorTargetYaw (+ (Variables|Default|GetDoorInitialYaw) (Variables|Default|GetDoorTargetYaw)))
  (if (Math|Boolean|Equal(Boolean) (Utilities|IsValid (Variables|Default|GetPressurePlate)) false) ; CPP\nif (!PressurePlate)
    (Development|PrintString (Utilities|String|BuildString(Name) "Error: " (Utilities|GetObjectName (Components|GetOwner)) "None" " has the OpenDoorBP component but PressurePlate is Null") false true "(R=1.000000,G=0.000000,B=0.000000,A=1.000000)")
    (else
      (Variables|Default|SetActorThatOpensDoor (Game|Player|GetPlayerPawn 0)))))

(event EventTick
  (params (DeltaSeconds :type Float%20%28single-precision%29))
  (if (and (Utilities|IsValid (Variables|Default|GetPressurePlate)) (Collision|IsOverlappingActor (Variables|Default|GetPressurePlate) (Variables|Default|GetActorThatOpensDoor) :!class /Script/Engine.Actor)) ; CPP\nif (PressurePlate && PressurePlate->IsOverlappingActor(ActorThatOpens))
    (CallFunction|OpenDoor DeltaSeconds)
    (Variables|Default|SetDoorLastOpened (Utilities|Time|GetTimeSeconds))
    (elif (> (- (Utilities|Time|GetTimeSeconds) (Variables|Default|GetDoorLastOpened)) (Variables|Default|GetDoorClosedDelay)) ; CPP\nif ((GetWorld()->GetTimeSeconds() - DoorLastOpened) >= DoorClosedDelay)
      (CallFunction|CloseDoor DeltaSeconds))))

(fn OpenDoor
  (params (DeltaTime :type Float%20%28single-precision%29))
  (Variables|Default|SetDoorCurrentYaw (Math|Float|Lerp (Variables|Default|GetDoorCurrentYaw) (Variables|Default|GetDoorTargetYaw) (* DeltaTime (Variables|Default|GetDoorOpenSpeed))))
  (Variables|Default|SetDoorRotation (Transformation|GetActorRotation (Components|GetOwner)))
  (Variables|Default|SetDoorRotation (Math|Rotator|MakeRotator 0.0 0.0 (Variables|Default|GetDoorCurrentYaw)))
  (Transformation|SetActorRotation (Components|GetOwner) (Variables|Default|GetDoorRotation)))

(fn CloseDoor
  (params (DeltaTime :type Float%20%28single-precision%29))
  (Variables|Default|SetDoorCurrentYaw (Math|Float|Lerp (Variables|Default|GetDoorCurrentYaw) (Variables|Default|GetDoorInitialYaw) (* DeltaTime (Variables|Default|GetDoorCloseSpeed))))
  (Variables|Default|SetDoorRotation (Transformation|GetActorRotation (Components|GetOwner)))
  (Variables|Default|SetDoorRotation (Math|Rotator|MakeRotator 0.0 0.0 (Variables|Default|GetDoorCurrentYaw)))
  (Transformation|SetActorRotation (Components|GetOwner) (Variables|Default|GetDoorRotation)))